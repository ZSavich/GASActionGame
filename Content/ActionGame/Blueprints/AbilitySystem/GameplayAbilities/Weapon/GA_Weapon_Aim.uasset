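; Weapon aiming gameplay ability that applies an aim camera modifier to the player's camera while active.
; On activation it adds the modifier class through the PlayerCameraManager and stores the instance, or ends immediately if the controller or camera manager is invalid.
; It then waits for the Event.Weapon.Aiming.Ended gameplay event to end itself, and removes the stored modifier when the ability ends.
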(event Ability|EventActivateAbility
  (bind _returnvalue (Ability|GetActorInfo))
  (Utilities|IsValid (.playercontroller _returnvalue)
    (:Is%20Valid
      (bind _playercameramanager (Variables|/Script/Engine.PlayerController|GetPlayerCameraManager (.playercontroller _returnvalue))
        (:then
          (bind _returnvalue_2 (Game|Player|AddNewCameraModifier _playercameramanager (Variables|Default|GetAimCameraModifierClass)))
          (Variables|Default|SetAimCameraModifier _returnvalue_2)
          (Ability|Tasks|WaitGameplayEvent "(TagName=\"Event.Weapon.Aiming.Ended\")" 0
            (:EventReceived
              (Ability|EndAbility))))
        (:else
          (Ability|EndAbility :!label _label))))
    (:Is%20Not%20Valid
      (goto _label))))

(event Ability|EventOnEndAbility
  (params (bWasCancelled :type Boolean))
  (bind _returnvalue (Ability|GetActorInfo))
  (Utilities|IsValid (.playercontroller _returnvalue)
    (:Is%20Valid
      (bind _playercameramanager (Variables|/Script/Engine.PlayerController|GetPlayerCameraManager (.playercontroller _returnvalue))
        (:then
          (bind _aimcameramodifier (Variables|Default|GetAimCameraModifier)
            (:then
              (Game|Player|RemoveCameraModifier _playercameramanager _aimcameramodifier))
            (:else)))
        (:else)))))