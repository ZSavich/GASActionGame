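; Gameplay ability for automatic weapon hip fire, configured by the equipped weapon's static data.
; Activation plays the attack montage and starts a looping timer at the fire rate, presumably driving Shot.
; Each shot line-traces from the muzzle along control rotation with debug drawing, applying the weapon's damage effect through the hit actor's ability system.
; The attack-ended event or montage finishing ends the ability, clearing the timer.
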(event Custom|Shot
  (bind _returnvalue (Class|AGGameplayAbilityInventory|GetEquippedWeaponStaticData))
  (bind _returnvalue_2 (Class|AGGameplayAbilityInventory|GetEquippedWeaponActor))
  (bind _returnvalue_3 (Ability|GetActorInfo))
  (bind _returnvalue_4 (Class|WeaponItemActor|GetMuzzleLocation _returnvalue_2))
  (Utilities|IsValid _returnvalue_2
    (:Is%20Valid
      (Utilities|IsValid (.playercontroller _returnvalue_3)
        (:Is%20Valid
          (bind (_outhit _returnvalue_5) (Collision|LineTraceByChannel _returnvalue_4 (+ _returnvalue_4 (* (Pawn|GetControlRotation (.playercontroller _returnvalue_3) :!class /Script/Engine.Controller) (Variables|Default|GetShotDuration))) "TraceTypeQuery1" false 0 "ForDuration"))
          (if _returnvalue_5
            (Utilities|IsValid (Ability|GetAbilitySystemComponent (.HitActor (Collision|BreakHitResult _outhit)))
              (:Is%20Valid
                (Utilities|IsValid _returnvalue
                  (:Is%20Valid
                    (GameplayEffects|ApplyGameplayEffectToSelf :self (Ability|GetAbilitySystemComponent (.HitActor (Collision|BreakHitResult _outhit))) :GameplayEffectClass (Variables|/Script/GASActionGame.WeaponStaticData|GetDamageEffect _returnvalue) :Level 1.0))
                  (:Is%20Not%20Valid
                    (Ability|EndAbility)))))))
        (:Is%20Not%20Valid
          (Ability|EndAbility :!label _label))))
    (:Is%20Not%20Valid
      (goto _label))))

(event Ability|EventOnEndAbility
  (params (bWasCancelled :type Boolean))
  (Utilities|Time|ClearandInvalidateTimerbyHandle (Variables|Default|GetFireTimer)))

(event Ability|EventActivateAbilityFromEvent
  (params (EventData :type Gameplay%20Event%20Data%20Structure%20%28by%20ref%29))
  (bind _returnvalue (Class|AGGameplayAbilityInventory|GetEquippedWeaponStaticData))
  (Utilities|IsValid _returnvalue
    (:Is%20Valid
      (|PlayMontageandWaitProxy "None" (Variables|/Script/GASActionGame.WeaponStaticData|GetAttackMontage _returnvalue) 1.0 "None" true 1.0 0.0
        (:then
          (bind _returnvalue_2 (Utilities|Time|SetTimerbyEvent (EventDispatchers|CreateEvent :!event Custom|Shot) (/ 1.0 (Variables|/Script/GASActionGame.WeaponStaticData|GetFireRate _returnvalue)) true))
          (Variables|Default|SetFireTimer _returnvalue_2)
          (Ability|Tasks|WaitGameplayEvent "(TagName=\"Event.Weapon.Attack.Ended\")" 0
            (:EventReceived
              (Ability|EndAbility))))
        (:OnCompleted
          (Ability|EndAbility :!label _label))
        (:OnInterrupted
          (goto _label))
        (:OnCancelled
          (goto _label))))))