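; Gameplay ability that fires a single shot from the equipped weapon.
; Activation plays the weapon's attack montage and waits for the Event.Weapon.Shoot gameplay event to trigger the shot.
; The shot traces from weapon to focus, plays weapon effects and applies the weapon's effect spec to a hit actor's Ability System Component.
; The ability ends when the montage finishes or breaks off, or when the shot finds no valid target.
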(event Custom|Shot
  (bind _shotduration (Variables|Default|GetShotDuration))
  (bind (_outhitresult _returnvalue) (Class|AGGameplayAbilityCombat|GetWeapontoFocusTraceResult _shotduration "TraceTypeQuery3"))
  (bind _hitactor (Collision|BreakHitResult _outhitresult))
  (bind _returnvalue_2 (Ability|GetAbilitySystemComponent _hitactor))
  (Class|WeaponItemActor|PlayWeaponEffects (Class|AGGameplayAbilityInventory|GetEquippedWeaponActor) _outhitresult)
  (if _returnvalue
    (Utilities|IsValid _returnvalue_2
      (:Is%20Valid
        (GameplayEffects|ApplyGameplayEffectSpecToSelf _returnvalue_2 (Class|AGGameplayAbilityCombat|GetWeaponEffectSpec _outhitresult)))
      (:Is%20Not%20Valid
        (Ability|EndAbility :!label _label)))
    (else
      (goto _label))))

(event Ability|EventActivateAbilityFromEvent
  (params (EventData :type Gameplay%20Event%20Data%20Structure%20%28by%20ref%29))
  (bind _returnvalue (Class|AGGameplayAbilityInventory|GetEquippedWeaponStaticData))
  (Utilities|IsValid _returnvalue
    (:Is%20Valid
      (|PlayMontageandWaitProxy "None" (Variables|/Script/GASActionGame.WeaponStaticData|GetAttackMontage _returnvalue) 1.0 "None" true 1.0 0.0
        (:then
          (Ability|Tasks|WaitGameplayEvent "(TagName=\"Event.Weapon.Shoot\")" 0
            (:EventReceived
              (CallFunction|Shot))))
        (:OnCompleted
          (Ability|EndAbility :!label _label))
        (:OnBlendOut
          (goto _label))
        (:OnInterrupted
          (goto _label))
        (:OnCancelled
          (goto _label))))))